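; Big enemy that moves along the X axis, patrolling with random waits until PawnSensing spots the player.
; It then chases to firing range, or fires in place if the player is in cover, and resumes patrol beyond RunAwayDistance.
; AttackPlayer locks movement and fires minigun bursts of pitch-jittered bullets, then cools down, reloads and rechecks range.
; Tick turns it toward the player outside patrol and cooldown; damage destroys it at zero health.
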(event `self.ReceiveBeginPlay`
  (bind _returnvalue (`GameplayStatics.GetActorOfClass` "/Game/Player/PlayerZD_BP.PlayerZD_BP_C"))
  (set `self.Player` _returnvalue)
  (`self.MovePatrol`))

(event `MovePatrol`
  (bind _returnvalue_x (`KismetMathLibrary.BreakVector` (`self.K2_GetActorLocation`)))
  (if (`self.OnPatrol`)
    (if (`self.LockMovement`)
      (`KismetSystemLibrary.Delay` 0.2)
      (`self.MovePatrol`)
      (else
        (`|AIMoveTo` self (`KismetMathLibrary.MakeVector` (+ _returnvalue_x (* (`self.MoveDistance`) (`self.RigthOrLeft`)))) null :!label _label
          (:`OnSuccess`
            (`/Engine/EditorBlueprintResources/StandardMacros.FlipFlop`
              (:`A`
                (set `self.RigthOrLeft` (* (`self.RigthOrLeft`) -1.0)))
              (:`B`
                (set `self.RigthOrLeft` (* (`self.RigthOrLeft`) 1.0))))
            (`KismetSystemLibrary.Delay` (`KismetMathLibrary.RandomFloatInRange` 0.1 (`self.MaxTimeWait`)))
            (goto _label)))))))

(event `self.ReceiveAnyDamage`
  (params (Damage :type "Float (single-precision)") (DamageType :type "DamageType Object Reference") (InstigatedBy :type "Controller Object Reference") (DamageCauser :type "Actor Object Reference"))
  (bind _output_get (set `self.Health` (- (`self.Health`) Damage)))
  (`/Engine/EditorBlueprintResources/StandardMacros.CompareFloat` _output_get
    (:`==`
      _)
    (:`<`
      _))
  (`self.K2_DestroyActor`))

(event `CheckDistance`
  (bind _returnvalue_x (`KismetMathLibrary.BreakVector` (`self.K2_GetActorLocation`)))
  (bind _runawaydistance (`self.RunAwayDistance`))
  (bind _returnvalue_x_2 (`KismetMathLibrary.BreakVector` (`self.K2_GetActorLocation` (`GameplayStatics.GetPlayerCharacter` 0))))
  (`/Engine/EditorBlueprintResources/StandardMacros.CompareFloat` _returnvalue_x (+ _returnvalue_x_2 _runawaydistance) :!label _label_2
    (:`>`
      (set `self.OnPatrol` true)
      (`self.MovePatrol`))
    (:`==`
      (if (`self.LockMovement`) :!label _label_3
        (if (`self.CooldownGun`) :!label _label_4
          (`KismetSystemLibrary.Delay` 0.2)
          (`self.CheckDistance`)
          (else
            (`self.AttackPlayer`)))
        (elif (`/Game/Player/PlayerZD_BP.InCover` (`self.Player`))
          (goto _label_4)
          (else
            (`|AIMoveTo` self (0.0 0.0 0.0) (`self.Player`) (`self.DistanceFromPlayer`) :!label _label_5
              (:`OnSuccess`
                (if (`self.CooldownGun`)
                  (`self.CheckDistance`)
                  (else
                    (`self.AttackPlayer`))))
              (:`OnFail`
                (`KismetSystemLibrary.Delay` 0.2)
                (goto _label_5)))))))
    (:`<`
      (`/Engine/EditorBlueprintResources/StandardMacros.CompareFloat` _returnvalue_x (- _returnvalue_x_2 _runawaydistance)
        (:`>`
          (goto _label_3))
        (:`==`
          (goto _label_3))
        (:`<`
          (set `self.OnPatrol` true)
          (`self.MovePatrol`))))))

(event `self.PawnSensing.OnSeePawn`
  (params (Pawn :type "Pawn Object Reference"))
  (if (== Pawn (`self.Player`))
    (set `self.OnPatrol` false)
    (goto _label_2)))

(event `AttackPlayer`
  (bind _returnvalue_x (`KismetMathLibrary.BreakVector` (`self.K2_GetActorLocation`)))
  (bind _returnvalue_x_2 (`KismetMathLibrary.BreakVector` (`self.K2_GetActorLocation`)))
  (bind _arrow1 (`self.Arrow1`))
  (bind _returnvalue_x_3 (`KismetMathLibrary.BreakVector` (`self.K2_GetActorLocation` (`GameplayStatics.GetPlayerCharacter` 0))))
  (bind (_returnvalue_roll _returnvalue_pitch _returnvalue_yaw) (`KismetMathLibrary.BreakRotator` (`SceneComponent.K2_GetComponentRotation` _arrow1)))
  (bind _returnvalue_x_4 (`KismetMathLibrary.BreakVector` (`self.K2_GetActorLocation` (`GameplayStatics.GetPlayerCharacter` 0))))
  (set `self.LockMovement` true)
  (bind _returnvalue (`|SpawnActorFromClass` "/Game/Hazards/EnemyBullet.EnemyBullet_C" (`KismetMathLibrary.MakeTransform` (`SceneComponent.K2_GetComponentLocation` _arrow1) (`KismetMathLibrary.MakeRotator` _returnvalue_roll (+ _returnvalue_pitch (`KismetMathLibrary.RandomFloatInRange` -5.0 5.0)) _returnvalue_yaw) (0.25 0.25 0.25)) "Undefined" "OverrideRootScale" null null :!label _label_6))
  (set `/Game/Hazards/EnemyBullet.BulletDamage` (`self.EnemyDamage`) _returnvalue)
  (`/Game/Hazards/EnemyBullet.KillBullet` _returnvalue)
  (bind _output_get (set `self.Ammo` (- (`self.Ammo`) 1)))
  (`/Engine/EditorBlueprintResources/StandardMacros.CompareInt` _output_get
    (:`>`
      (`KismetSystemLibrary.Delay` (`self.FireRate`))
      (goto _label_6))
    (:`==`
      _)
    (:`<`
      _))
  (set `self.CooldownGun` true)
  (`KismetSystemLibrary.Delay` (`self.CooldownMinigun`))
  (set `self.Ammo` 20)
  (set `self.CooldownGun` false)
  (`/Engine/EditorBlueprintResources/StandardMacros.CompareFloat` _returnvalue_x_2 (+ _returnvalue_x_4 (`self.DistanceFromPlayer`))
    (:`>`
      (set `self.LockMovement` false)
      (`self.CheckDistance`))
    (:`==`
      (`KismetSystemLibrary.Delay` 0.2 :!label _label_7)
      (`self.AttackPlayer`))
    (:`<`
      (`/Engine/EditorBlueprintResources/StandardMacros.CompareFloat` _returnvalue_x (- _returnvalue_x_3 (`self.DistanceFromPlayer`))
        (:`>`
          (goto _label_7))
        (:`==`
          (goto _label_7))
        (:`<`
          (set `self.LockMovement` false)
          (`self.CheckDistance`))))))

(event `self.ReceiveTick`
  (params (DeltaSeconds :type "Float (single-precision)"))
  (`self.RotateCharacter`))

(event `RotateCharacter`
  (bind _returnvalue_x (`KismetMathLibrary.BreakVector` (`self.K2_GetActorLocation`)))
  (bind _returnvalue_x_2 (`KismetMathLibrary.BreakVector` (`self.K2_GetActorLocation` (`self.Player`))))
  (if (`self.OnPatrol`)
    _
    (elif (not (`self.CooldownGun`))
      (`/Engine/EditorBlueprintResources/StandardMacros.CompareFloat` _returnvalue_x _returnvalue_x_2
        (:`>`
          (`self.K2_SetActorRelativeRotation` (struct :`Yaw` 180.0)))
        (:`<`
          (`self.K2_SetActorRelativeRotation` (struct)))))))

(fn `UserConstructionScript`)