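; Dog enemy AI that patrols along the X axis, chases the player on sight and is destroyed when its health runs out.
; Patrol chains AIMoveTo steps with random waits, using a FlipFlop to reverse direction on alternate arrivals.
; PawnSensing starts a distance-check loop that resumes patrol when the player leaves an X-range, otherwise closes in.
; Attacks use a short forward line trace with debug drawing, applying damage on a one-second cooldown.
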(event `self.ReceiveBeginPlay`
  (bind _returnvalue (`GameplayStatics.GetActorOfClass` "/Game/Player/PlayerZD_BP.PlayerZD_BP_C"))
  (set `self.Player` _returnvalue)
  (`self.MovePatrol`))

(event `MovePatrol`
  (bind _returnvalue_x (`KismetMathLibrary.BreakVector` (`self.K2_GetActorLocation`)))
  (if (`self.OnPatrol`)
    (`|AIMoveTo` self (`KismetMathLibrary.MakeVector` (+ _returnvalue_x (* (`self.MoveDistance`) (`self.RigthOrLeft`)))) null :!label _label
      (:`OnSuccess`
        (`/Engine/EditorBlueprintResources/StandardMacros.FlipFlop`
          (:`A`
            (set `self.RigthOrLeft` (* (`self.RigthOrLeft`) -1.0)))
          (:`B`
            (set `self.RigthOrLeft` (* (`self.RigthOrLeft`) 1.0))))
        (`KismetSystemLibrary.Delay` (`KismetMathLibrary.RandomFloatInRange` 0.1 (`self.MaxTimeWait`)))
        (goto _label)))))

(event `self.ReceiveAnyDamage`
  (params (Damage :type "Float (single-precision)") (DamageType :type "DamageType Object Reference") (InstigatedBy :type "Controller Object Reference") (DamageCauser :type "Actor Object Reference"))
  (bind _output_get (set `self.Health` (- (`self.Health`) Damage)))
  (`/Engine/EditorBlueprintResources/StandardMacros.CompareFloat` _output_get
    (:`==`
      _)
    (:`<`
      _))
  (`self.K2_DestroyActor`))

(event `CheckDistance`
  (bind _returnvalue_x (`KismetMathLibrary.BreakVector` (`self.K2_GetActorLocation`)))
  (bind _runawaydistance (`self.RunAwayDistance`))
  (bind _returnvalue_x_2 (`KismetMathLibrary.BreakVector` (`self.K2_GetActorLocation` (`GameplayStatics.GetPlayerCharacter` 0))))
  (`/Engine/EditorBlueprintResources/StandardMacros.CompareFloat` _returnvalue_x (+ _returnvalue_x_2 _runawaydistance) :!label _label_2
    (:`>`
      (set `self.OnPatrol` true)
      (`self.MovePatrol`))
    (:`==`
      (if (`self.LockMovement`) :!label _label_3
        (if (`self.CooldownGun`)
          (`KismetSystemLibrary.Delay` 0.2)
          (`self.CheckDistance`)
          (else
            (`self.AttackPlayer`)))
        (else
          (`|AIMoveTo` self (0.0 0.0 0.0) (`self.Player`) (`self.DistanceFromPlayer`) :!label _label_4
            (:`OnSuccess`
              (if (`self.CooldownGun`)
                (`self.CheckDistance`)
                (else
                  (`self.AttackPlayer`))))
            (:`OnFail`
              (`KismetSystemLibrary.Delay` 0.2)
              (goto _label_4))))))
    (:`<`
      (`/Engine/EditorBlueprintResources/StandardMacros.CompareFloat` _returnvalue_x (- _returnvalue_x_2 _runawaydistance)
        (:`>`
          (goto _label_3))
        (:`==`
          (goto _label_3))
        (:`<`
          (set `self.OnPatrol` true)
          (`self.MovePatrol`))))))

(event `self.PawnSensing.OnSeePawn`
  (params (Pawn :type "Pawn Object Reference"))
  (if (== Pawn (`self.Player`))
    (set `self.OnPatrol` false)
    (goto _label_2)))

(event `AttackPlayer`
  (bind _returnvalue (`self.K2_GetActorLocation`))
  (bind _player (`self.Player`))
  (set `self.LockMovement` true)
  (bind _outhit (`KismetSystemLibrary.LineTraceSingle` :`Start` _returnvalue :`End` (+ _returnvalue (* (`SceneComponent.GetForwardVector` (`self.CapsuleComponent`)) 200.0)) :`TraceChannel` "TraceTypeQuery1" :`DrawDebugType` "ForDuration"))
  (if (== _player (`.HitActor` (`GameplayStatics.BreakHitResult` _outhit)))
    (`GameplayStatics.ApplyDamage` _player (`self.EnemyDamage`)))
  (`self.Cooldown`)
  (set `self.LockMovement` false)
  (`self.CheckDistance`))

(event `Cooldown`
  (set `self.CooldownGun` true)
  (`KismetSystemLibrary.Delay` 1.0)
  (set `self.CooldownGun` false))

(fn `UserConstructionScript`)