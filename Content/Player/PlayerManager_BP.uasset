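; Player manager that persists the player's upgrades, health, currency, position and fake-store usage in a SaveSlot1 save game.
; On BeginPlay it finds PlayerZD_BP, then loads slot "1", replaying upgrade calls and copying values onto the player, or saves a blank slot.
; The SaveGame event writes current state back if the slot exists, using the object cached on load, which the new-slot branch never sets.
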(event `self.ReceiveBeginPlay`
  (bind _as_save_slot_1 (`self.As Save Slot 1`))
  (bind _as_save_slot_1_2 (`self.As Save Slot 1`))
  (bind _as_save_slot_1_3 (`self.As Save Slot 1`))
  (bind _as_save_slot_1_4 (`self.As Save Slot 1`))
  (bind _player (`self.Player`))
  (bind _player_2 (`self.Player`))
  (bind _player_3 (`self.Player`))
  (bind _returnvalue (`GameplayStatics.GetActorOfClass` "/Game/Player/PlayerZD_BP.PlayerZD_BP_C"))
  (set `self.Player` _returnvalue)
  (bind _returnvalue_2 (`GameplayStatics.DoesSaveGameExist` "1"))
  (if _returnvalue_2
    (bind _returnvalue_3 (`GameplayStatics.LoadGameFromSlot` "1"))
    (bind _assave_slot_1 (cast `/Game/Interact/SaveZone/SaveSlot1` _returnvalue_3))
    (set `self.As Save Slot 1` _assave_slot_1)
    (if (`/Game/Interact/SaveZone/SaveSlot1.Muzzle` _as_save_slot_1_2)
      (`/Game/Player/PlayerZD_BP.ImprovedMuzzle` _player))
    (if (`/Game/Interact/SaveZone/SaveSlot1.Bullet Velocity` _as_save_slot_1_2)
      (`/Game/Player/PlayerZD_BP.HighVelocityBullets` _player))
    (if (`/Game/Interact/SaveZone/SaveSlot1.Bullet Damage` _as_save_slot_1_2)
      (`/Game/Player/PlayerZD_BP.HighCaliberBullets` _player))
    (set `/Game/Player/PlayerZD_BP.ImprovedArmor?` (`/Game/Interact/SaveZone/SaveSlot1.Armor` _as_save_slot_1_2) _player)
    (if (`/Game/Interact/SaveZone/SaveSlot1.Laser` _as_save_slot_1_2)
      (`/Game/Player/PlayerZD_BP.LaserSight` _player))
    (set `/Game/Player/PlayerZD_BP.SuperLight?` (`/Game/Interact/SaveZone/SaveSlot1.LightPU` _as_save_slot_1_3) _player_2)
    (set `/Game/Player/PlayerZD_BP.DashPower?` (`/Game/Interact/SaveZone/SaveSlot1.DashPU` _as_save_slot_1_3) _player_2)
    (if (`/Game/Interact/SaveZone/SaveSlot1.JumpPU` _as_save_slot_1_3)
      (`/Game/Player/PlayerZD_BP.DoubleJump` _player_2))
    (set `/Game/Player/PlayerZD_BP.HealthSaved` (`/Game/Interact/SaveZone/SaveSlot1.CurrentHealth` _as_save_slot_1_4) _player_3)
    (set `/Game/Player/PlayerZD_BP.SavedPosition` (`/Game/Interact/SaveZone/SaveSlot1.FinalLocation` _as_save_slot_1_4) _player_3)
    (set `/Game/Player/PlayerZD_BP.Currency` (`/Game/Interact/SaveZone/SaveSlot1.TotalCurrency` _as_save_slot_1_4) _player_3)
    (set `/Game/Player/PlayerZD_BP.SavedPosition?` (`/Game/Interact/SaveZone/SaveSlot1.SavedPosition?` _as_save_slot_1_4) _player_3)
    (set `self.Fake Store 1 Used?` (`/Game/Interact/SaveZone/SaveSlot1.FakeStore1Used?` _as_save_slot_1))
    (set `self.Fake Store 2 Used?` (`/Game/Interact/SaveZone/SaveSlot1.FakeStore2Used?` _as_save_slot_1))
    (set `self.Fake Store 3 Used?` (`/Game/Interact/SaveZone/SaveSlot1.FakeStore3Used?` _as_save_slot_1))
    (else
      (bind _returnvalue_4 (`GameplayStatics.CreateSaveGameObject` "/Game/Interact/SaveZone/SaveSlot1.SaveSlot1_C"))
      (`GameplayStatics.SaveGameToSlot` _returnvalue_4 "1"))))

(event `SaveGame`
  (bind _player (`self.Player`))
  (bind _as_save_slot_1 (`self.As Save Slot 1`))
  (bind _player_2 (`self.Player`))
  (bind _as_save_slot_1_2 (`self.As Save Slot 1`))
  (bind _as_save_slot_1_3 (`self.As Save Slot 1`))
  (bind _player_3 (`self.Player`))
  (bind _as_save_slot_1_4 (`self.As Save Slot 1`))
  (bind _returnvalue (`GameplayStatics.DoesSaveGameExist` "1"))
  (if _returnvalue
    (set `/Game/Interact/SaveZone/SaveSlot1.Muzzle` (`/Game/Player/PlayerZD_BP.ImprovedMuzzle?` _player_2) _as_save_slot_1_2)
    (set `/Game/Interact/SaveZone/SaveSlot1.Bullet Damage` (`/Game/Player/PlayerZD_BP.HighCaliberBullets?` _player_2) _as_save_slot_1_2)
    (set `/Game/Interact/SaveZone/SaveSlot1.Bullet Velocity` (`/Game/Player/PlayerZD_BP.HighVelocityBullets?` _player_2) _as_save_slot_1_2)
    (set `/Game/Interact/SaveZone/SaveSlot1.Armor` (`/Game/Player/PlayerZD_BP.ImprovedArmor?` _player_2) _as_save_slot_1_2)
    (set `/Game/Interact/SaveZone/SaveSlot1.Laser` (`/Game/Player/PlayerZD_BP.LaserSight?` _player_2) _as_save_slot_1_2)
    (set `/Game/Interact/SaveZone/SaveSlot1.DashPU` (`/Game/Player/PlayerZD_BP.DashPower?` _player_3) _as_save_slot_1_3)
    (set `/Game/Interact/SaveZone/SaveSlot1.JumpPU` (`/Game/Player/PlayerZD_BP.DoubleJump?` _player_3) _as_save_slot_1_3)
    (set `/Game/Interact/SaveZone/SaveSlot1.LightPU` (`/Game/Player/PlayerZD_BP.SuperLight?` _player_3) _as_save_slot_1_3)
    (set `/Game/Interact/SaveZone/SaveSlot1.CurrentHealth` (`/Game/Player/PlayerZD_BP.HealthSaved` _player) _as_save_slot_1_4)
    (set `/Game/Interact/SaveZone/SaveSlot1.FinalLocation` (`/Game/Player/PlayerZD_BP.SavedPosition` _player) _as_save_slot_1_4)
    (set `/Game/Interact/SaveZone/SaveSlot1.TotalCurrency` (`/Game/Player/PlayerZD_BP.Currency` _player) _as_save_slot_1_4)
    (set `/Game/Interact/SaveZone/SaveSlot1.FakeStore1Used?` (`self.Fake Store 1 Used?`) _as_save_slot_1)
    (set `/Game/Interact/SaveZone/SaveSlot1.FakeStore2Used?` (`self.Fake Store 2 Used?`) _as_save_slot_1)
    (set `/Game/Interact/SaveZone/SaveSlot1.FakeStore3Used?` (`self.Fake Store 3 Used?`) _as_save_slot_1)
    (set `/Game/Interact/SaveZone/SaveSlot1.SavedPosition?` (`/Game/Interact/SaveZone/SaveSlot1.SavedPosition?` (`self.As Save Slot 1`)) _as_save_slot_1)
    (`GameplayStatics.SaveGameToSlot` _as_save_slot_1 "1")))

(fn `UserConstructionScript`)