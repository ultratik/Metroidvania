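; Player character Blueprint for side-on movement, handling walking, jumping, crouching, aiming and a toggled cover state.
; Movement runs along local X and flips Sphere to face travel, but is blocked while aiming or in cover.
; Cover and aim use MoveComponentTo to shift the character between two Y offsets.
; Gamepad axes and keys snap Arrow1 to upward and diagonal aim angles; AimWithMouse, uncalled here, points it at the cursor hit.
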(event `self.ReceiveTick`
  (params (DeltaSeconds :type "Float (single-precision)")))

(event `InputAxis|Move Right and Left`
  (params (AxisValue :type "Float (single-precision)"))
  (bind _sphere (`self.Sphere`))
  ;[1 1 1 1 100] Movement Actions
  ;;[1 1 1 1 70] Sides Movement
  (if (`self.Aiming?`)
    _
    (elif (not (`self.InCover`))
      (`self.K2_AddActorLocalOffset` (`KismetMathLibrary.MakeVector` (* AxisValue (`self.MoveSpeed`))))
      (`/Engine/EditorBlueprintResources/StandardMacros.CompareFloat` AxisValue
        (:`>`
          (`SceneComponent.K2_SetRelativeRotation` _sphere (struct) false false))
        (:`<`
          (`SceneComponent.K2_SetRelativeRotation` _sphere (struct :`Yaw` 180.0) false false))))))

(event `InputAction|Aim`
  (params (Key :type "Key Structure"))
  (bind (_returnvalue_x _returnvalue_y _returnvalue_z) (`KismetMathLibrary.BreakVector` (`self.K2_GetActorLocation`)))
  (bind (_returnvalue_x_2 _returnvalue_y_2 _returnvalue_z_2) (`KismetMathLibrary.BreakVector` (`self.K2_GetActorLocation`)))
  ;[1 1 1 1 100] Aiming
  ;;[1 1 1 1 70] Aim Input
  (:`Pressed`
    (if (`self.InCover`)
      (set `self.Aiming?` true)
      (`KismetSystemLibrary.MoveComponentTo` (`self.RootComponent`) (`KismetMathLibrary.MakeVector` _returnvalue_x (`self.CoverOffsetPositive`) _returnvalue_z))
      (else
        (set `self.Aiming?` true))))
  (:`Released`
    (if (`self.InCover`)
      (set `self.Aiming?` false)
      (`KismetSystemLibrary.MoveComponentTo` (`self.RootComponent`) (`KismetMathLibrary.MakeVector` _returnvalue_x_2 (`self.CoverOffsetNegative`) _returnvalue_z_2))
      (else
        (set `self.Aiming?` false)))))

(event `InputAction|Jump`
  (params (Key :type "Key Structure"))
  ;[1 1 1 1 100] Movement Actions
  ;;[1 1 1 1 70] Jumping
  (:`Pressed`
    (`self.Jump`)))

(event `InputAxis|ControllerAimY`
  (params (AxisValue :type "Float (single-precision)"))
  (bind _arrow1 (`self.Arrow1`))
  ;[1 1 1 1 100] Aiming
  ;;[1 1 1 1 70] Aim Direction Gamepad
  (`/Engine/EditorBlueprintResources/StandardMacros.CompareFloat` AxisValue
    (:`>`
      (`/Engine/EditorBlueprintResources/StandardMacros.CompareFloat` AxisValue 0.9
        (:`>`
          (`SceneComponent.K2_SetWorldRotation` _arrow1 (struct :`Pitch` 90.0) false false))))
    (:`==`
      (`SceneComponent.K2_SetRelativeRotation` :`self` _arrow1))))

(event `InputAxis|Crouch`
  (params (AxisValue :type "Float (single-precision)"))
  ;[1 1 1 1 100] Movement Actions
  ;;[1 1 1 1 70] Crouching
  (`/Engine/EditorBlueprintResources/StandardMacros.CompareFloat` AxisValue
    (:`>`
      (`/Engine/EditorBlueprintResources/StandardMacros.CompareFloat` AxisValue 0.3
        (:`>`
          (`self.Crouch`)
          (set `self.MoveSpeed` 5.0))))
    (:`==`
      (`self.UnCrouch`)
      (set `self.MoveSpeed` 10.0))))

(event `InputAction|AimD Up`
  (params (Key :type "Key Structure"))
  (bind _arrow1 (`self.Arrow1`))
  ;[1 1 1 1 100] Aiming
  ;;[1 1 1 1 70] Aim Direction Keyboard
  (:`Pressed`
    (`SceneComponent.K2_SetWorldRotation` _arrow1 (struct :`Pitch` 90.0) false false))
  (:`Released`
    (`SceneComponent.K2_SetRelativeRotation` :`self` _arrow1)))

(event `InputAction|Cover`
  (params (Key :type "Key Structure"))
  (bind (_returnvalue_x _returnvalue_y _returnvalue_z) (`KismetMathLibrary.BreakVector` (`self.K2_GetActorLocation`)))
  (bind (_returnvalue_x_2 _returnvalue_y_2 _returnvalue_z_2) (`KismetMathLibrary.BreakVector` (`self.K2_GetActorLocation`)))
  ;[1 1 1 1 100] Movement Actions
  ;;[1 1 1 1 70] Take Cover
  (:`Pressed`
    (if (not (`self.Aiming?`))
      (`/Engine/EditorBlueprintResources/StandardMacros.FlipFlop`
        (:`A`
          (set `self.InCover` true)
          (`KismetSystemLibrary.MoveComponentTo` (`self.RootComponent`) (`KismetMathLibrary.MakeVector` _returnvalue_x_2 (`self.CoverOffsetNegative`) _returnvalue_z_2)))
        (:`B`
          (set `self.InCover` false)
          (`KismetSystemLibrary.MoveComponentTo` (`self.RootComponent`) (`KismetMathLibrary.MakeVector` _returnvalue_x (`self.CoverOffsetPositive`) _returnvalue_z)))))))

(event `InputAxis|ControllerAimX`
  (params (AxisValue :type "Float (single-precision)"))
  (bind _returnvalue (`self.GetInputAxisValue`))
  (bind _returnvalue_2 (`self.GetInputAxisValue`))
  (bind _arrow1 (`self.Arrow1`))
  ;[1 1 1 1 100] Aiming
  ;;[1 1 1 1 70] Aim Direction Gamepad
  (`/Engine/EditorBlueprintResources/StandardMacros.CompareFloat` AxisValue
    (:`>`
      (if (`self.Aiming?`)
        (`SceneComponent.K2_SetRelativeRotation` :`self` (`self.Sphere`)))
      (`/Engine/EditorBlueprintResources/StandardMacros.CompareFloat` _returnvalue_2 0.3
        (:`>`
          (`/Engine/EditorBlueprintResources/StandardMacros.CompareFloat` _returnvalue_2 0.9
            (:`<`
              (`SceneComponent.K2_SetWorldRotation` _arrow1 (struct :`Pitch` 45.0) false false))))))
    (:`==`
      (`SceneComponent.K2_SetRelativeRotation` :`self` _arrow1))
    (:`<`
      (if (`self.Aiming?`)
        (`SceneComponent.K2_SetRelativeRotation` (`self.Sphere`) (struct :`Yaw` 180.0) false false))
      (`/Engine/EditorBlueprintResources/StandardMacros.CompareFloat` _returnvalue 0.3
        (:`>`
          (`/Engine/EditorBlueprintResources/StandardMacros.CompareFloat` _returnvalue 0.9
            (:`<`
              (`SceneComponent.K2_SetWorldRotation` _arrow1 (struct :`Pitch` 135.0) false false))))))))

(event `InputAction|AimD UpRight`
  (params (Key :type "Key Structure"))
  (bind _arrow1 (`self.Arrow1`))
  ;[1 1 1 1 100] Aiming
  ;;[1 1 1 1 70] Aim Direction Keyboard
  (:`Pressed`
    (`SceneComponent.K2_SetWorldRotation` _arrow1 (struct :`Pitch` 45.0) false false))
  (:`Released`
    (`SceneComponent.K2_SetRelativeRotation` :`self` _arrow1)))

(event `InputAction|AimD UpLeft`
  (params (Key :type "Key Structure"))
  (bind _arrow1 (`self.Arrow1`))
  ;[1 1 1 1 100] Aiming
  ;;[1 1 1 1 70] Aim Direction Keyboard
  (:`Pressed`
    (`SceneComponent.K2_SetWorldRotation` _arrow1 (struct :`Pitch` 135.0) false false))
  (:`Released`
    (`SceneComponent.K2_SetRelativeRotation` :`self` _arrow1)))

(event `AimWithMouse`
  (bind _hitresult (`PlayerController.GetHitResultUnderCursorByChannel` (`GameplayStatics.GetPlayerController` 0) "TraceTypeQuery2" true))
  (bind (_returnvalue_roll _returnvalue_pitch _returnvalue_yaw) (`KismetMathLibrary.BreakRotator` (`KismetMathLibrary.FindLookAtRotation` (`self.K2_GetActorLocation`) (`.ImpactPoint` (`GameplayStatics.BreakHitResult` _hitresult)))))
  (set `PlayerController.bShowMouseCursor` false (`GameplayStatics.GetPlayerController` 0))
  (`SceneComponent.K2_SetWorldRotation` (`self.Arrow1`) (`KismetMathLibrary.MakeRotator` 0.0 _returnvalue_pitch _returnvalue_yaw) false false)
  (`KismetSystemLibrary.DrawDebugSphere` (`.ImpactPoint` (`GameplayStatics.BreakHitResult` _hitresult))))

(fn `UserConstructionScript`)